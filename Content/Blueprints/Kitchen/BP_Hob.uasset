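; BP_Hob is a kitchen hob with an adjustable power level for cooking.
; Changes to the HobButton value are stored as the current power percent and shown on the temperature bar of its WB_HobTemperature widget component.
; A box trigger sends begin and end cooking-machine collision messages to overlapping actors, passing the hob itself, and prints debug text.
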(event OnComponentBeginOverlap(Box)
  (params (OverlappedComponent :type Primitive%20Component%20Object%20Reference) (OtherActor :type Actor%20Object%20Reference) (OtherComp :type Primitive%20Component%20Object%20Reference) (OtherBodyIndex :type Integer) (bFromSweep :type Boolean) (SweepResult :type Hit%20Result%20Structure%20%28by%20ref%29))
  (Class|BPICookableItem|OnCollisionBeginwithCookingMachine(Message) OtherActor self)
  (Development|PrintString "Hit"))

(event OnComponentEndOverlap(Box)
  (params (OverlappedComponent :type Primitive%20Component%20Object%20Reference) (OtherActor :type Actor%20Object%20Reference) (OtherComp :type Primitive%20Component%20Object%20Reference) (OtherBodyIndex :type Integer))
  (Class|BPICookableItem|OnCollisionEndwithCookingMachine(Message) OtherActor self)
  (Development|PrintString "UnHit"))

(event Custom|OnButtonValueChanged_Event
  (params (ButtonValue :type Float%20%28double-precision%29))
  (bind _aswb_hob_temperature (Utilities|Casting|CastToWB_HobTemperature (UserInterface|GetWidget (Variables|Components|GetTemperature%20Widget)))
    (:then
      (bind _output_get (Variables|Default|SetCurrentPowerPercent ButtonValue))
      (Progress|SetPercent (Variables|/Game/Blueprints/Kitchen/WB_HobTemperature.WB_HobTemperature_C|GetTemperatureBar _aswb_hob_temperature) _output_get))
    (:CastFailed
      (Development|PrintString "Cast to WB_HobTemperature failed"))))

(event EventBeginPlay
  (EventDispatchers|AssignOnButtonValueChanged (Variables|Default|GetHobButton) (delegate Custom|OnButtonValueChanged_Event)))

(fn ConstructionScript)