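; BP_Fridge is a fridge Blueprint with a pivoting door and a grab component for motion controller interaction.
; RotateDoor yaws the DoorPivot toward a given position, using Atan2 on the XY offset from the pivot, and applies it as relative rotation.
; The call feeding it the controller's location is disconnected, so grabbing currently only prints a debug string.
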(event OnGrabbed(GrabComponent)
  (Development|PrintString "Grab"))

(fn ConstructionScript)

(fn RotateDoor
  (params (position :type Vector))
  (bind _doorpivot (Variables|Default|GetDoorPivot))
  (bind _returnvalue (Transformation|GetWorldLocation _doorpivot))
  (bind _returnvalue_2 (- position _returnvalue))
  (Transformation|SetRelativeRotation _doorpivot (Math|Rotator|MakeRotator 0.0 0.0 (Class|KismetMathLibrary|DegAtan2 (.y _returnvalue_2) (.x _returnvalue_2))) false false))