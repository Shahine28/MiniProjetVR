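; BP_Plate is a plate actor on which burger ingredients are stacked.
; Its overlap sphere marks ingredients in or out of range, keeping snapped ones marked on exit.
; SnapIngredient places each at the stack's top and tracks it in IngredientsSnapped, which also serves removal and last-ingredient checks.
; CombineBurger unsnaps the bottom ingredient, but its attach loop fires only on the last index, targeting an out-of-range element.
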(event OnComponentBeginOverlap(Sphere)
  (params (OverlappedComponent :type Primitive%20Component%20Object%20Reference) (OtherActor :type Actor%20Object%20Reference) (OtherComp :type Primitive%20Component%20Object%20Reference) (OtherBodyIndex :type Integer) (bFromSweep :type Boolean) (SweepResult :type Hit%20Result%20Structure%20%28by%20ref%29))
  (bind _asbp_burger_ingredient (Utilities|Casting|CastToBP_BurgerIngredient OtherActor))
  (Default|MarkasinRange _asbp_burger_ingredient self)
  (Development|PrintString (Utilities|GetDisplayName _asbp_burger_ingredient)))

(event OnComponentEndOverlap(Sphere)
  (params (OverlappedComponent :type Primitive%20Component%20Object%20Reference) (OtherActor :type Actor%20Object%20Reference) (OtherComp :type Primitive%20Component%20Object%20Reference) (OtherBodyIndex :type Integer))
  (bind _asbp_burger_ingredient (Utilities|Casting|CastToBP_BurgerIngredient OtherActor))
  (if (not (Utilities|Array|ContainsItem (Variables|Default|GetIngredientsSnapped) _asbp_burger_ingredient))
    (Default|UnmarkasinRange _asbp_burger_ingredient)))

(event Custom|CombineBurger
  (bind _ingredientssnapped (Variables|Default|GetIngredientsSnapped))
  (for (_array_element _array_index) _ingredientssnapped
    (if (== (Utilities|Array|LastIndex _ingredientssnapped) _array_index)
      (Transformation|AttachActorToActor (Utilities|Array|Get(acopy) _ingredientssnapped (+ _array_index 1)) _array_element "None" "KeepRelative" "KeepRelative" "KeepRelative" true)))
  (Default|UnsnapfromPlate (Utilities|Array|Get(acopy) _ingredientssnapped)))

(event Custom|CallSnap
  (bind _testingredient (Variables|Default|GetTestIngredient)
    (:then
      (CallFunction|SnapIngredient _testingredient))
    (:else)))

(event Custom|SnapIngredient
  (params (Ingredient :type BP%20Burger%20Ingredient%20Object%20Reference))
  (Default|SnaptoPlate Ingredient (CallFunction|GetTopPosition))
  (Utilities|Array|AddUnique (Variables|Default|GetIngredientsSnapped) Ingredient))

(fn ConstructionScript)

(fn GetTopPosition
  (bind _ingredientssnapped (Variables|Default|GetIngredientsSnapped))
  (if (Utilities|Array|IsEmpty _ingredientssnapped)
    (return (Transformation|GetWorldLocation (Variables|Default|GetSnapPosition)))
    (else
      (return (Default|GetTopWorldPosition (Utilities|Array|Get(acopy) _ingredientssnapped (- (Utilities|Array|Length _ingredientssnapped) 1)))))))

(fn IsLastIngredient
  (params (Ingredient :type BP%20Burger%20Ingredient%20Object%20Reference%20%28by%20ref%29))
  (bind _ingredientssnapped (Variables|Default|GetIngredientsSnapped))
  (return (and (Utilities|Array|ContainsItem _ingredientssnapped Ingredient) (== (Utilities|Array|FindItem _ingredientssnapped Ingredient) (Utilities|Array|LastIndex _ingredientssnapped)))))

(fn RemovefromPlate
  (params (Ingredient :type BP%20Burger%20Ingredient%20Object%20Reference))
  (bind _ingredientssnapped (Variables|Default|GetIngredientsSnapped))
  (if (Utilities|Array|ContainsItem _ingredientssnapped Ingredient)
    (Utilities|Array|RemoveItem _ingredientssnapped Ingredient)
    (Default|UnsnapfromPlate Ingredient)))