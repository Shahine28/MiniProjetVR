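; BP_BurgerIngredient is a VR-grabbable burger ingredient that stacks on a plate and can remove itself once from its fridge by Id.
; When dropped with a plate in range, it asks that plate to snap it.
; Snapping disables physics, changes the grab type and aligns its bottom marker to the given stack top, exposing its own top position.
; Grabbing a plated ingredient succeeds only for the last one; others are released.
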(event OnDropped(GrabComponent)
  (if (not (Variables|Default|GetIsOnPlate))
    (bind _plate (Variables|Default|GetPlate)
      (:then
        (Default|SnapIngredient _plate self))
      (:else))))

(event OnGrabbed(GrabComponent)
  (params (MotionController :type Motion%20Controller%20Component%20Object%20Reference))
  (bind _self self)
  (bind _grabcomponent (Variables|Default|GetGrabComponent))
  (if (Variables|Default|GetIsOnPlate)
    (bind _plate (Variables|Default|GetPlate)
      (:then
        (bind _result (Default|IsLastIngredient _plate _self))
        (if _result
          (Default|RemovefromPlate _plate _self)
          (Default|TryGrab _grabcomponent (Variables|/Game/VRTemplate/Blueprints/GrabComponent.GrabComponent_C|GetMotionControllerRef _grabcomponent))
          (else
            (Default|TryRelease _grabcomponent))))
      (:else))))

(fn ConstructionScript
  (Variables|Default|SetDefaultGrabType (Variables|/Game/VRTemplate/Blueprints/GrabComponent.GrabComponent_C|GetGrabType (Variables|Default|GetGrabComponent)))
  (Variables|Default|SetMeshDefaultOffset (Variables|/Script/Engine.SceneComponent|GetRelativeLocation (Variables|Default|GetStaticMesh))))

(fn GetTopWorldPosition
  (return (Transformation|GetWorldLocation (Variables|Default|GetTopPosition))))

(fn SnaptoPlate
  (params (PlateTopPosition :type Vector))
  (bind _returnvalue (Transformation|GetActorScale3D))
  (bind _downposition (Variables|Default|GetDownPosition))
  (bind _staticmesh (Variables|Default|GetStaticMesh))
  (bind _relativelocation (Variables|/Script/Engine.SceneComponent|GetRelativeLocation _downposition))
  (bind _returnvalue_2 (* (.z _relativelocation) (.x _returnvalue)))
  (bind _returnvalue_3 (- (.z PlateTopPosition) _returnvalue_2))
  (bind _returnvalue_4 (Math|Vector|MakeVector (.x PlateTopPosition) (.y PlateTopPosition) _returnvalue_3))
  (Variables|/Game/VRTemplate/Blueprints/GrabComponent.GrabComponent_C|SetGrabType (Variables|Default|GetGrabComponent) "NewEnumerator3")
  (Physics|SetSimulatePhysics _staticmesh false)
  (Development|PrintString (Utilities|String|ToString(Vector) _returnvalue_4))
  (Transformation|SetActorLocation _returnvalue_4 false true)
  (Transformation|SetActorRotation "0, 0, 0")
  (Transformation|SetWorldLocation _staticmesh (+ _returnvalue_4 (Variables|Default|GetMeshDefaultOffset)) false true)
  (Transformation|SetRelativeRotation (Variables|Default|GetStaticMesh) "0, 0, 0" false false)
  (Variables|Default|SetIsOnPlate true))

(fn UnsnapfromPlate
  (Variables|/Game/VRTemplate/Blueprints/GrabComponent.GrabComponent_C|SetGrabType (Variables|Default|GetGrabComponent) (Variables|Default|GetDefaultGrabType))
  (Physics|SetSimulatePhysics (Variables|Default|GetStaticMesh) true)
  (Variables|Default|SetIsOnPlate false))

(fn MarkasinRange
  (params (Plate :type BP%20Plate%20Object%20Reference))
  (Variables|Default|SetPlate Plate))

(fn UnmarkasinRange
  (Variables|Default|SetPlate 0))

(fn RemoveIngredientfromFridge
  (if (not (Variables|Default|GetisRemove))
    (Default|RemoveFoodfromFridge (Variables|Default|GetFridge) (Variables|Default|GetId))
    (Variables|Default|SetisRemove true)))