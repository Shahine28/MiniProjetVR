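; Kitchen monitor that shows the current orders as tickets on a WBP_KitchenScreen hosted in its Widget component.
; On BeginPlay it binds to the OrderManager's added, completed and failed events, then caches the screen widget.
; Each new order spawns a WBP_OrderTicket and adds it to the screen.
; Completed and failed orders are handled alike: the ticket is looked up by order ID and removed from its parent.
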(event Custom|OnOrderAdded_Event
  (params (NewOrder :type Active%20Order%20Structure%20%28by%20ref%29))
  (bind _returnvalue (UserInterface|CreateWidget "/Game/Blueprints/Orders/WBP_OrderTicket.WBP_OrderTicket_C" 0 NewOrder))
  (Default|AddOrder (Variables|Default|GetKitchenScreen) _returnvalue))

(event Custom|OnOrderCompleted_Event
  (params (OrderID :type Integer))
  (bind _oder (Default|GetOrder (Variables|Default|GetKitchenScreen) OrderID))
  (Widget|RemovefromParent _oder))

(event Custom|OnOrderFailed_Event
  (params (OrderID :type Integer))
  (bind _oder (Default|GetOrder (Variables|Default|GetKitchenScreen) OrderID))
  (Widget|RemovefromParent _oder))

(event EventBeginPlay
  (EventDispatchers|AssignOnOrderAdded (Variables|Default|GetOrderManager) (delegate Custom|OnOrderAdded_Event))
  (EventDispatchers|AssignOnOrderCompleted (Variables|Default|GetOrderManager) (delegate Custom|OnOrderCompleted_Event))
  (EventDispatchers|AssignOnOrderFailed (Variables|Default|GetOrderManager) (delegate Custom|OnOrderFailed_Event))
  (bind _aswbp_kitchen_screen (Utilities|Casting|CastToWBP_KitchenScreen (UserInterface|GetUserWidgetObject (Variables|Default|GetWidget))))
  (Variables|Default|SetKitchenScreen _aswbp_kitchen_screen))

(fn ConstructionScript)