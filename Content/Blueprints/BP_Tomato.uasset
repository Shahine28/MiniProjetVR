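; BP_Tomato is a tomato item that can be snapped onto and released from a plate.
; It overrides its parent's snap and unsnap functions, calling the parent and toggling physics simulation on its static mesh.
; On snap, it teleports the mesh to the plate top, lowered by the DownPosition component's relative Z so that this reference point lines up with the plate surface.
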(fn ConstructionScript)

(fn SnaptoPlate
  (params (PlateTopPosition :type Vector :default "0, 0, 0"))
  (bind (_x _y _z) (Math|Vector|BreakVector PlateTopPosition))
  (bind _staticmesh (Variables|Default|GetStaticMesh))
  (Physics|SetSimulatePhysics _staticmesh false)
  (|CallParentFunction PlateTopPosition)
  (Transformation|SetWorldLocation _staticmesh (Math|Vector|MakeVector _x _y (- _z (.z (Variables|/Script/Engine.SceneComponent|GetRelativeLocation (Variables|Default|GetDownPosition))))) false true))

(fn UnsnapfromPlate
  (|CallParentFunction)
  (Physics|SetSimulatePhysics (Variables|Default|GetStaticMesh) true))